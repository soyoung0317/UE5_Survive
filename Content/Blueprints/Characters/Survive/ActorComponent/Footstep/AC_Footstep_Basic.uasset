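; Footstep actor component that plays a surface-dependent sound at the ground under a character's left or right foot.
; ExecuteFootstepLogic traces briefly down from the chosen foot socket on the supplied skeletal mesh to read the surface type and hit location.
; On a hit, it plays that foot's matching cue quietly at the impact point.
; Wood, Water, Snow and Flash have no cues, and Dirt has only a right-foot default cue.
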(fn `Execute_Footstep_Logic`
  (params (`SkeletalMesh Component` :type "SkeletalMeshComponent Object Reference") (`Is RightFoot` :type Boolean))
  (bind (_returnvalue _location _is_detect) (`self.SurfaceType Detection` `SkeletalMesh Component` `Is RightFoot`))
  (if _is_detect
    (`self.Play Footstep Sound` _returnvalue _location `Is RightFoot`)))

(fn `Get Notify Location Based on Socket`
  (params (`Skeletal Mesh Component` :type "SkeletalMeshComponent Object Reference") (`Is RightFoot` :type Boolean))
  (returns (`Socket Location` :type "Vector Structure"))
  (return (`KismetMathLibrary.SelectVector` (`SceneComponent.GetSocketLocation` `Skeletal Mesh Component` "foot_r") (`SceneComponent.GetSocketLocation` `Skeletal Mesh Component` "foot_l") `Is RightFoot`)))

(fn `Play Footstep Sound`
  (params (`Surface Type` :type "EPhysicalSurface Enum" :default "SurfaceType_Default") (location :type "Vector Structure") (`Is RightFoot` :type Boolean))
  (if `Is RightFoot`
    (`GameplayStatics.PlaySoundAtLocation` (select `EPhysicalSurface` `Surface Type` :`SurfaceType_Default` "/Game/Blueprints/ResourcePack/Sound/Footstep/Default/Sound_R_Default_Footstep_Cue.Sound_R_Default_Footstep_Cue" :`SurfaceType1` "/Game/Blueprints/ResourcePack/Sound/Footstep/Grass/Sound_R_Grass_Footstep_Cue.Sound_R_Grass_Footstep_Cue" :`SurfaceType2` "/Game/Blueprints/ResourcePack/Sound/Footstep/Rock/Sound_R_Rock_Footstep_Cue.Sound_R_Rock_Footstep_Cue" :`SurfaceType5` "/Game/Blueprints/ResourcePack/Sound/Footstep/Sand/Sound_R_Sand_Footstep_Cue.Sound_R_Sand_Footstep_Cue" :`SurfaceType6` "/Game/Blueprints/ResourcePack/Sound/Footstep/Default/Sound_R_Default_Footstep_Cue.Sound_R_Default_Footstep_Cue" :!type "SoundBase Object Reference") location (struct) 0.05 1.0 0.0 null null null null)
    (else
      (`GameplayStatics.PlaySoundAtLocation` (select `EPhysicalSurface` `Surface Type` :`SurfaceType_Default` "/Game/Blueprints/ResourcePack/Sound/Footstep/Default/Sound_L_Default_Footstep_Cue.Sound_L_Default_Footstep_Cue" :`SurfaceType1` "/Game/Blueprints/ResourcePack/Sound/Footstep/Grass/Sound_L_Grass_Footstep_Cue.Sound_L_Grass_Footstep_Cue" :`SurfaceType2` "/Game/Blueprints/ResourcePack/Sound/Footstep/Rock/Sound_L_Rock_Footstep_Cue.Sound_L_Rock_Footstep_Cue" :`SurfaceType5` "/Game/Blueprints/ResourcePack/Sound/Footstep/Sand/Sound_L_Sand_Footstep_Cue.Sound_L_Sand_Footstep_Cue" :!type "SoundBase Object Reference") location (struct) 0.05 1.0 0.0 null null null null))))

(fn `SurfaceType Detection`
  (params (`Skeletal Mesh Component` :type "SkeletalMeshComponent Object Reference") (`Is RightFoot` :type Boolean))
  (returns (ReturnValue :type "EPhysicalSurface Enum") (Location :type "Vector Structure") (`Is Detect` :type Boolean))
  (bind _socket_location (`self.Get Notify Location Based on Socket` `Skeletal Mesh Component` `Is RightFoot`))
  (bind (_outhit _returnvalue) (`KismetSystemLibrary.LineTraceSingle` _socket_location (- _socket_location (0.0 0.0 50.0)) "TraceTypeQuery1"))
  (if _returnvalue
    (return (`GameplayStatics.GetSurfaceType` _outhit) (`.Location` (`GameplayStatics.BreakHitResult` _outhit)) _returnvalue)
    (else
      (return "SurfaceType_Default" (0.0 0.0 0.0) false))))