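; Actor component that detects interactable actors in view of the locally controlled pawn and shows an interact prompt on them.
; On BeginPlay it adds the interaction mapping context and starts a looping timer that line-traces from the active camera.
; Hits implementing BPI_CanInteract become the current target, with an attached prompt button using the interface's text and location; losing the target clears both.
; The IA_TryInteract input event is still empty.
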(event `self.ReceiveBeginPlay`
  ;[0 0 0] Initialization of input mapping on local controlled pawns, and initialize the can interact trace
  (`/Engine/EditorBlueprintResources/StandardMacros.IsValid` (`.Controller` (`/Game/Blueprints/Core/BlueprintMacroLibrary/BML_Generic_Component.Get Controller`))
    (:`Is Valid`
      (if (`Pawn.IsLocallyControlled` (`/Game/Blueprints/Core/BlueprintMacroLibrary/BML_Generic_Component.Get Pawn`))
        (`self.Initialize`)))))

(event `Initialize`
  ;[0 0 0] Initialization of input mapping on local controlled pawns, and initialize the can interact trace
  (`/Game/Blueprints/Characters/Survive/ActorComponent/Movement/MovementFunc/BF_Locomotion.Link Input Mapping Context` false false (`/Game/Blueprints/Core/BlueprintMacroLibrary/BML_Generic_Component.Get Player Controller`) "/Game/Blueprints/Characters/Survive/Input/InputMapping/IMC_Interaction.IMC_Interaction")
  (`self.Start Can Interact Trace`))

(event `Start Can Interact Trace`
  (`KismetSystemLibrary.K2_SetTimerDelegate` (delegate `LineTraceInteraction`) 0.1 true))

(event `LineTraceInteraction`
  (bind (_outhit _is_hit _hitactor) (`/Game/Blueprints/Core/BlueprintFunctionLibrary/BFL_Generic.Trace From Active Camera` (`/Game/Blueprints/Core/BlueprintMacroLibrary/BML_Generic_Component.Get Player Controller`) "TraceTypeQuery3" (`|MakeArray` null :!type "Actor Object Reference") 100.0 1500.0 "ForDuration"))
  (`self.Handle Interaction Logic` _is_hit _hitactor))

(event `EnhancedInput|/Game/Blueprints/Characters/Survive/Input/Interactions/IA_TryInteract`
  (params (ActionValue :type Boolean) (ElapsedSeconds :type "Float (double-precision)") (TriggeredSeconds :type "Float (double-precision)") (InputAction :type "InputAction Object Reference" :default "/Game/Blueprints/Characters/Survive/Input/Interactions/IA_TryInteract.IA_TryInteract")))

(fn `Cancel Interaction`
  (`self.Able to Interact with this actor`
    (:`then`
      (set `self.Able to Interact with this actor` null)
      (bind _active_interact_button_ (`self.Active Interact Button `)
        (:`then`
          (`Actor.K2_DestroyActor` _active_interact_button_)
          (set `self.Active Interact Button ` null))
        (:`else`)))
    (:`else`)))

(fn `Handle Interaction Logic`
  (params (`Is Hit` :type Boolean) (`Hit Actor` :type "Actor Object Reference"))
  (bind _able_to_interact_with_this_actor (`self.Able to Interact with this actor`))
  (if `Is Hit`
    (if (`KismetSystemLibrary.DoesImplementInterface` `Hit Actor` "/Game/Blueprints/Core/Interfaces/BPI_CanInteract.BPI_CanInteract_C")
      (bind _able_to_interact_with_this_actor_2 (`self.Able to Interact with this actor`)
        (:`then`
          (if (not (== _able_to_interact_with_this_actor_2 (`local.Hit Actor`)))
            (`self.Cancel Interaction`)
            (set `self.Able to Interact with this actor` (`local.Hit Actor`) :!label _label) ; Setting able to interact reference
            (bind _interact_text (message `/Game/Blueprints/Core/Interfaces/BPI_CanInteract.Get Interact Text` _able_to_interact_with_this_actor (`/Game/Blueprints/Core/BlueprintMacroLibrary/BML_Generic_Component.Get Player Controller`)))
            (bind _relative_interaction_text (message `/Game/Blueprints/Core/Interfaces/BPI_CanInteract.Get Relative Interact TextLocation` _able_to_interact_with_this_actor))
            (bind _returnvalue (`|SpawnActorFromClass` "/Game/Blueprints/Widget/Interaction/BP_CanInteract_Button.BP_CanInteract_Button_C" (`KismetMathLibrary.MakeTransform` _relative_interaction_text) "AlwaysSpawn" "MultiplyWithRoot" null _interact_text null))
            (bind _output_get (set `self.Active Interact Button ` _returnvalue))
            (`Actor.K2_AttachToActor` _output_get (`self.Able to Interact with this actor`) "None" "KeepRelative" "KeepRelative" "KeepRelative" true)))
        (:`else`
          (bind _active_interact_button_ (`self.Active Interact Button `)
            (:`then`
              (`Actor.K2_DestroyActor` _active_interact_button_)
              (set `self.Active Interact Button ` null)
              (goto _label))
            (:`else`
              (goto _label)))))
      (else
        (`self.Cancel Interaction` :!label _label_2)))
    (else
      (goto _label_2))))