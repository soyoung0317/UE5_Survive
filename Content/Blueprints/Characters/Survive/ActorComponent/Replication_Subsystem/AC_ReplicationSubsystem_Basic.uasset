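; Actor component that replicates animation montage playback for a survival character across the network.
; The montage plays locally first, then a server event triggers a multicast that plays it on every machine except the locally controlled one, avoiding a double play.
; The stop-montage event is an empty stub, and its MontageStop call is left unconnected.
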(event `self.Initialize Stop Multicast Montage`)

(event `self.Initialize Multicast Motage`
  (params (`Montage to Play` :type "AnimMontage Object Reference"))
  ;[0 0 0] Play the animation first, after that, call to the server
  (`self.Event Play Montage` `Montage to Play`)
  (`self.Event Play Montage in Server` `Montage to Play`))

(event `Event Play Montage in Server`
  (params (Montage :type "AnimMontage Object Reference"))
  ;[0 0 0] only the server is able to execute a multicast. call a multicast from server
  (`self.Evemt Multicast Montage to all client` Montage))

(event `Evemt Multicast Montage to all client`
  (params (Montage :type "AnimMontage Object Reference"))
  ;[0 0 0] play on ALL clients including server, except the local one, since that one is already playing
  (if (not (`Pawn.IsLocallyControlled` (`/Game/Blueprints/Core/BlueprintMacroLibrary/BML_Generic_Component.Get Character`)))
    (`self.Event Play Montage` Montage)))

(event `Event Play Montage`
  (params (Montage :type "AnimMontage Object Reference"))
  ;[0 0 0] play the actual montage
  (`|PlayMontage` (`/Game/Blueprints/Core/BlueprintMacroLibrary/BML_Generic_Component.Get CharacterMesh`) Montage))