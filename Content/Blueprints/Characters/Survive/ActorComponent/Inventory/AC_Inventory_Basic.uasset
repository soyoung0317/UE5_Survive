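; AC_Inventory_Basic is an inventory component that opens and closes the inventory screen from player input.
; BeginPlay links the IMC_UI mapping context, and the Enhanced Input action IA_Inventory toggles the active state.
; WBP_Inventory is created lazily on first open, then shown or collapsed rather than recreated.
; Each toggle also switches between Game-and-UI and Game-Only input modes and shows or hides the mouse cursor.
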(event `self.ReceiveBeginPlay`
  ;[0 0 0] Initialization of UI Controls
  (`parent.ReceiveBeginPlay`)
  (`/Game/Blueprints/Characters/Survive/ActorComponent/Movement/MovementFunc/BF_Locomotion.Link Input Mapping Context` false false (`/Game/Blueprints/Core/BlueprintMacroLibrary/BML_Generic_Component.Get Player Controller`) "/Game/Blueprints/Characters/Survive/Input/IMC_UI.IMC_UI"))

(event `EnhancedInput|/Game/Blueprints/Characters/Survive/Input/Actions/IA_Inventory`
  (params (ActionValue :type Boolean) (ElapsedSeconds :type "Float (double-precision)") (TriggeredSeconds :type "Float (double-precision)") (InputAction :type "InputAction Object Reference" :default "/Game/Blueprints/Characters/Survive/Input/Actions/IA_Inventory.IA_Inventory"))
  (:`Started`
    (if (`self.Is Inventory Active`)
      (`self.Enable Inventory Widget` false)
      (else
        (`self.WBP_Inventory`
          (:`then`
            _)
          (:`else`
            (`self.Create Inventory `)))
        (`self.Enable Inventory Widget` true)))))

(event `Create Inventory`
  (bind _returnvalue (`|CreateWidget` "/Game/Blueprints/Widget/Inventory/WBP_Inventory.WBP_Inventory_C"))
  (bind _output_get (set `self.WBP_Inventory` _returnvalue))
  (`UserWidget.AddToViewport` _output_get 0))

(event `Enable Inventory Widget`
  (params (Enable :type Boolean))
  (bind _asplayer_controller (`/Game/Blueprints/Core/BlueprintMacroLibrary/BML_Generic_Component.Get Player Controller`))
  (bind _output_get (set `self.Is Inventory Active` Enable))
  (if _output_get
    (`Widget.SetVisibility` (`self.WBP_Inventory`) "Visible")
    (`WidgetBlueprintLibrary.SetInputMode_GameAndUIEx` _asplayer_controller (`self.WBP_Inventory`)) ; game and ui 로 해야 더이상의 mapping이 안된다 -> 인벤토리 띄워서 점프하는거 x
    (set `PlayerController.bShowMouseCursor` true _asplayer_controller)
    (else
      (`Widget.SetVisibility` (`self.WBP_Inventory`) "Collapsed")
      (`WidgetBlueprintLibrary.SetInputMode_GameOnly` _asplayer_controller)
      (set `PlayerController.bShowMouseCursor` false _asplayer_controller))))