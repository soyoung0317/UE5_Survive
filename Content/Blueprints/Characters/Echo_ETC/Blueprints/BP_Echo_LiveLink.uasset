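; BP_Echo_LiveLink is an Echo character Blueprint whose graphs configure the body and hair, with a name that points to Live Link use.
; The construction script calls ProxyConstruct, which turns on in-editor animation updates for the Body mesh.
; It then uses UseGroomAssets to either assign hair and eyebrow grooms with their bindings, or set a skinned hair mesh instead.
; BeginPlay and Tick contain no logic.
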(event `ProxyConstruct`
  (`SkeletalMeshComponent.SetUpdateAnimationInEditor` (`self.Body`) true))

(event `self.ReceiveBeginPlay`)

(fn `UserConstructionScript`
  (`self.ProxyConstruct`)
  (`|ExecutionSequence`
    (:`then_0`
      ;[1 1 1] Hair
      (if (`self.useGroomAssets`)
        (`GroomComponent.SetGroomAsset` (`self.HairGroom`) "/Game/Blueprints/Characters/Echo/Hair/Hair_S_UpdoBuns.Hair_S_UpdoBuns")
        (`GroomComponent.SetGroomAsset` (`self.EyebrowGroom`) "/Game/Blueprints/Characters/Echo/Hair/Eyebrows_L_Echo.Eyebrows_L_Echo")
        (`GroomComponent.SetBindingAsset` (`self.EyebrowGroom`) "/Game/Blueprints/Characters/Echo/Hair/Eyebrows.Eyebrows")
        (`GroomComponent.SetBindingAsset` (`self.HairGroom`) "/Game/Blueprints/Characters/Echo/Hair/Hair.Hair")
        (else
          (`SkinnedMeshComponent.SetSkinnedAssetAndUpdate` (`self.HairMesh`) "/Game/Blueprints/Characters/Echo/Meshes/Echo_Hair.Echo_Hair" true))))))