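; Interactable light prop whose point light is toggled through a replicated on/off state.
; Interact flips IsOn, and its RepNotify sets the PointLight component active or inactive to match.
; The interaction functions request server-controlled interaction and supply prompt text at a fixed offset above the actor.
; CanInteract always returns false, whichever controller is passed.
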(event `/Game/Blueprints/Core/Interfaces/BPI_Interact.Interact`
  (params (Controller :type "Controller Object Reference"))
  (if (`self.Is On`)
    (set `self.Is On` false)
    (else
      (set `self.Is On` true))))

(fn `Can Interact`
  (params (Controller :type "Controller Object Reference"))
  (returns (Can :type Boolean))
  (return false))

(fn `Get Interact Text`
  (params (Controller :type "Controller Object Reference"))
  (returns (`Interact Text` :type Text))
  (return (`self.Interact Text`)))

(fn `Get Relative Interact TextLocation`
  (returns (`Relative Interaction Text` :type "Vector Structure"))
  (return (0.0 0.0 100.0)))

(fn `OnRep_Is On`
  (`ActorComponent.SetActive` (`self.PointLight`) (`self.Is On`) false))

(fn `Should Server control the interaction`
  (returns (`Server should execute interaction` :type Boolean))
  (return true))

(fn `UserConstructionScript`
  (`parent.UserConstructionScript`))