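; A fire prop for the interaction system that switches a point light and Niagara effect on and off.
; Interact toggles IsOn under server-controlled interaction, and its RepNotify activates or deactivates both components, setting the light white or black.
; It supplies interact text at a fixed offset of 100 on Z, but CanInteract always returns false.
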(event `self.Interact`
  (params (Controller :type "Controller Object Reference"))
  (if (`self.Is On`)
    (set `self.Is On` false)
    (else
      (set `self.Is On` true))))

(fn `Can Interact`
  (params (Controller :type "Controller Object Reference"))
  (returns (Can :type Boolean))
  (return false))

(fn `Get Interact Text`
  (params (Controller :type "Controller Object Reference"))
  (returns (`Interact Text` :type Text))
  (return (`self.Interact Text`)))

(fn `Get Relative Interact TextLocation`
  (returns (`Relative Interaction Text` :type "Vector Structure"))
  (return (0.0 0.0 100.0)))

(fn `OnRep_Is On`
  (bind _pointlight (`self.PointLight`))
  (bind _pointlight_2 (`self.PointLight`))
  (bind _niagara (`self.Niagara`))
  (if (`self.Is On`)
    (`ActorComponent.SetActive` _pointlight_2 true false) ; on
    (`LightComponent.SetLightColor` _pointlight (struct :`R` 1.0 :`G` 1.0 :`B` 1.0 :`A` 1.0) true)
    (`ActorComponent.SetActive` _niagara true false)
    (else
      (`ActorComponent.SetActive` _pointlight_2 false false) ; off
      (`LightComponent.SetLightColor` :`self` _pointlight)
      (`ActorComponent.SetActive` _niagara false false))))

(fn `Should Server control the interaction`
  (returns (`Server should execute interaction` :type Boolean))
  (return true))

(fn `UserConstructionScript`
  (`parent.UserConstructionScript`))